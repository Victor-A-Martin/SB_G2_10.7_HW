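; BP_Movable is a pawn that wanders endlessly between random reachable navigation points within a fixed radius of itself.
; From BeginPlay, Move picks a point, snaps rotation toward it and runs AIMoveTo, restarting on success or failure.
; Overlapping a StaticMeshActor calls RotateFunction without a target.
; A 2D boundary check is defined but unused, and the movement input uses a zero direction.
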(event `self.ReceiveBeginPlay`
  (`self.Move`))

(event `self.Collision.OnComponentBeginOverlap`
  (params (OverlappedComponent :type "PrimitiveComponent Object Reference") (OtherActor :type "Actor Object Reference") (OtherComp :type "PrimitiveComponent Object Reference") (OtherBodyIndex :type Integer) (bFromSweep :type Boolean) (SweepResult :type "HitResult Structure (by ref)"))
  (cast `StaticMeshActor` OtherActor)
  (`self.RotateFunction` (0.0 0.0 0.0)))

(event `Move`
  (`self.AddMovementInput` (0.0 0.0 0.0) (`self.Speed`))
  (bind _output_get (set `self.TargetLocation` (`NavigationSystemV1.K2_GetRandomReachablePointInRadius` (`self.K2_GetActorLocation`) 500.0 null null)))
  (`self.RotateFunction` _output_get)
  (`|AIMoveTo` self (`self.TargetLocation`) null 0.5
    (:`OnSuccess`
      _)
    (:`OnFail`
      _))
  (`self.Move`))

(fn `Is Actor In Boundaries 2D`
  (params (`Min X` :type "Float (double-precision)") (`Max X` :type "Float (double-precision)") (`Min Y` :type "Float (double-precision)") (`Max Y` :type "Float (double-precision)"))
  (returns (ReturnValue :type Boolean))
  (bind (_returnvalue_x _returnvalue_y) (`KismetMathLibrary.BreakVector` (`self.K2_GetActorLocation`)))
  (return (and (`KismetMathLibrary.InRange_FloatFloat` _returnvalue_x `Min X` `Max X`) (`KismetMathLibrary.InRange_FloatFloat` _returnvalue_y `Min Y` `Max Y`))))

(fn `RotateFunction`
  (params (Target :type "Vector Structure (by ref)"))
  (`self.K2_SetActorRotation` (`KismetMathLibrary.FindLookAtRotation` (`self.K2_GetActorLocation`) Target)))

(fn `UserConstructionScript`)